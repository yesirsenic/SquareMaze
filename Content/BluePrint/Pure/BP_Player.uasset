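; BP_Player is a player Blueprint that handles running and jump audio; it contains no movement logic.
; WASD presses start the run sound behind an IsPlaying flag, and releases stop it once AnyKeyDown finds none of those keys held.
; Tick also stops the audio at zero velocity, without clearing IsPlaying.
; SpaceBar plays a 2D jump cue on every press, with no airborne check.
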(event EventBeginPlay)

(event Collision|EventActorBeginOverlap
  (params (OtherActor :type Actor%20Object%20Reference)))

(event EventTick
  (params (DeltaSeconds :type Float%20%28single-precision%29))
  (bind _audio (Variables|Default|GetAudio))
  (if (== (Math|Vector|VectorLength (Variables|/Script/Engine.MovementComponent|GetVelocity (Variables|Character|GetCharacterMovement))) 0.0)
    (if (Audio|Components|Audio|IsPlaying _audio)
      (Audio|Components|Audio|Stop _audio))))

(event Input|KeyboardEvents|SpaceBar
  (params (Key :type Key%20Structure :default "None"))
  (:Pressed
    (Audio|PlaySound2D "/Game/Resouces/Music/SFX/Jump_Cue.Jump_Cue" 1.0 1.0 0.0 0 0)))

(event Input|KeyboardEvents|W
  (params (Key :type Key%20Structure :default "None"))
  (:Pressed
    (CallFunction|PlayRunSound))
  (:Released
    (CallFunction|StopRunSound)))

(event Input|KeyboardEvents|D
  (params (Key :type Key%20Structure :default "None"))
  (:Pressed
    (CallFunction|PlayRunSound))
  (:Released
    (CallFunction|StopRunSound)))

(event Input|KeyboardEvents|A
  (params (Key :type Key%20Structure :default "None"))
  (:Pressed
    (CallFunction|PlayRunSound))
  (:Released
    (CallFunction|StopRunSound)))

(event Input|KeyboardEvents|S
  (params (Key :type Key%20Structure :default "None"))
  (:Pressed
    (CallFunction|PlayRunSound))
  (:Released
    (CallFunction|StopRunSound)))

(fn ConstructionScript
  (|CallParentFunction))

(fn PlayRunSound
  (if (not (Variables|Default|GetIs_Playing))
    (Audio|Components|Audio|Play (Variables|Default|GetAudio) 0.0)
    (Variables|Default|SetIs_Playing true)))

(fn StopRunSound
  (bind _move (CallFunction|AnyKeyDown))
  (if (not _move)
    (Audio|Components|Audio|Stop (Variables|Default|GetAudio))
    (Variables|Default|SetIs_Playing false)))

(fn AnyKeyDown
  (if (Game|Player|IsInputKeyDown (Game|GetPlayerController 0) "W")
    (return true)
    (elif (Game|Player|IsInputKeyDown (Game|GetPlayerController 0) "A")
      (return true)
      (elif (Game|Player|IsInputKeyDown (Game|GetPlayerController 0) "S")
        (return true)
        (elif (Game|Player|IsInputKeyDown (Game|GetPlayerController 0) "D")
          (return true)
          (else
            (return false)))))))